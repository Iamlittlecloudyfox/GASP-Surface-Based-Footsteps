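; Animation notify that plays a foley sound for its gameplay tag Event, with adjustable volume and pitch.
; FoleySoundSided resolves the foley bank and play location from the mesh and Side, and the bank maps the tag to a sound.
; Handplant events instead use DefaultBank at the mesh location, while notifies blending out always use a fixed side.
; The notify's display name comes from the tag's last segment.
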(fn ReceivedNotify
  (params (MeshComp :type Skeletal%20Mesh%20Component%20Object%20Reference) (Animation :type Anim%20Sequence%20Base%20Object%20Reference) (EventReference :type Anim%20Notify%20Event%20Reference%20Structure%20%28by%20ref%29))
  (bind _defaultbank (Variables|Default|GetDefaultBank))
  (bind _event (Variables|Default|GetEvent))
  (bind _sound (Default|GetSoundfromFoleyEvent _defaultbank _event))
  (if (not (Class|AnimNotifyLibrary|IsBlendingOut EventReference))
    (if (== (Variables|Default|GetEvent) "(TagName=\"Foley.Event.Handplant\")")
      (Utilities|IsValid _sound
        (:Is%20Valid
          (Audio|PlaySoundatLocation _sound (Transformation|GetWorldLocation MeshComp) "0, 0, 0" (Variables|Default|GetVolumeMultiplier) (Variables|Default|GetPitchMultiplier) 0.0 0 0 0 0)))
      (else
        (bind (_foleybank _location) (CallFunction|FoleySoundSided MeshComp (Variables|Default|GetSide)))
        (Utilities|IsValid _foleybank
          (:Is%20Valid
            (Audio|PlaySoundatLocation (.Sound (Default|GetSoundfromFoleyEvent _foleybank (Variables|Default|GetEvent))) _location "0, 0, 0" (Variables|Default|GetVolumeMultiplier) (Variables|Default|GetPitchMultiplier) 0.0 0 0 0 0)
            (return true)))))
    (else
      (bind (_foleybank_2 _location_2) (CallFunction|FoleySoundSided MeshComp "NewEnumerator4"))
      (Utilities|IsValid _foleybank_2
        (:Is%20Valid
          (Audio|PlaySoundatLocation (.Sound (Default|GetSoundfromFoleyEvent _foleybank_2 (Variables|Default|GetEvent))) _location_2 "0, 0, 0" (Variables|Default|GetVolumeMultiplier) (Variables|Default|GetPitchMultiplier) 0.0 0 0 0 0)
          (return true))))))

(fn GetNotifyName
  (bind _event (Variables|Default|GetEvent))
  (bind _returnvalue (GameplayTags|GetDebugStringfromGameplayTag _event))
  (bind _rights (Utilities|String|Split _returnvalue "." "IgnoreCase" "FromEnd"))
  (bind _result (Utilities|Text|FormatText "FoleyEvent: {Type}" _rights))
  (bind _returnvalue_2 (Utilities|String|ToString(Text) _result))
  (Development|PrintString _returnvalue_2)
  (return _returnvalue_2))